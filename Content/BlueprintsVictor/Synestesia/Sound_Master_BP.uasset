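; Sound emitter actor that plays a sound and turns its spectrum into visual pulses.
; Playback progress indexes Audio Synesthesia Constant-Q data for channel 0, writing each band in turn to the PC_Outline parameter collection's SoundRadius, alongside the source's SoundLoc, so the last band's radius remains.
; Tick reads that radius back and, above a threshold, spawns a sound-wave particle and Light actor at the source, throttled by a DoOnce reset after a short delay.
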(event `self.ReceiveBeginPlay`
  (`AudioComponent.SetSound` (`self.Audio`) (`self.New Sound`))
  (set `self.Duration` (`SoundBase.Duration` (`self.New Sound`)))
  (add `AudioComponent.OnAudioPlaybackPercent` (`self.Audio`) (delegate `PlaybackChange`))
  (`AudioComponent.Play` (`self.Audio`) 0.0))

(event `PlaybackChange`
  (params (PlayingSoundWave :type "SoundWave Object Reference") (PlaybackPercent :type "Float (double-precision)"))
  (set `self.PlayedTime` (* PlaybackPercent (`self.Duration`)))
  (for _array_element (`ConstantQNRT.GetNormalizedChannelConstantQAtTime` (`self.Constant_ref`) (`self.PlayedTime`) 0)
    (`|ExecutionSequence`
      (:`then_0`
        (`KismetMaterialLibrary.SetScalarParameterValue` "/Game/BlueprintsVictor/DarkWorldSystem/PC_Outline.PC_Outline" "SoundRadius" (+ (* _array_element 250.0) 100.0))
        (`KismetMaterialLibrary.SetVectorParameterValue` "/Game/BlueprintsVictor/DarkWorldSystem/PC_Outline.PC_Outline" "SoundLoc" (`KismetMathLibrary.Conv_VectorToLinearColor` (`SceneComponent.K2_GetComponentLocation` (`self.Audio`))))))))

(event `self.ReceiveTick`
  (params (DeltaSeconds :type "Float (single-precision)"))
  (bind _returnvalue (`KismetMaterialLibrary.GetScalarParameterValue` "/Game/BlueprintsVictor/DarkWorldSystem/PC_Outline.PC_Outline" "SoundRadius"))
  (if (> _returnvalue 280.0)
    (`/Engine/EditorBlueprintResources/StandardMacros.DoOnce` false :!label _label
      (:`Completed`
        (`GameplayStatics.SpawnEmitterAtLocation` "/Game/THE_GAME/ARTISTS/Niagara/MeepsSoundWaveeAdvanced.MeepsSoundWaveeAdvanced" (`SceneComponent.K2_GetComponentLocation` (`self.Audio`)) (struct) (0.8 0.8 2.0))
        (`|SpawnActorFromClass` "/Game/BlueprintsVictor/Light.Light_C" (`KismetMathLibrary.MakeTransform` (`SceneComponent.K2_GetComponentLocation` (`self.Audio`)) (struct) (3.0 3.0 3.0)) "Undefined" "OverrideRootScale" null null)
        (`KismetSystemLibrary.Delay` 0.3)
        (goto _label :!via `Reset`)))))

(fn `UserConstructionScript`)