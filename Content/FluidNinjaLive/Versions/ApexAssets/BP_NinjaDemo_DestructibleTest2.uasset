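; FluidNinja Live demo actor that breaks an APEX destructible box, either after play begins or when the player touches it.
; DMBox starts without gravity; if OverlapSensitive, a configurable trigger box waits for the player pawn to overlap, otherwise the sequence runs immediately.
; After an initial delay, the Gravity option enables falling and shortly applies small radius damage at the mesh's location with a configurable impulse to shatter it.
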(event `self.ReceiveBeginPlay`
  (bind _box (`self.Box`))
  (bind _dm_box (`self.DM_box`))
  (`PrimitiveComponent.SetEnableGravity` (`self.DM_box`) false)
  (if (`self.OverlapSensitive`)
    (add `PrimitiveComponent.OnComponentBeginOverlap` _box (delegate `Overlap`))
    (`BoxComponent.SetBoxExtent` _box (`self.OverlapBoxExtent`) true)
    (else
      (`KismetSystemLibrary.Delay` (`self.InitialDelay`) :!label _label)
      (if (`self.Gravity`)
        (`PrimitiveComponent.SetEnableGravity` _dm_box true)
        (`KismetSystemLibrary.Delay` 0.2)
        (`DestructibleComponent.ApplyRadiusDamage` _dm_box 1.0 (`SceneComponent.K2_GetComponentLocation` _dm_box) 5.0 (`self.ImpulseStrength`) false)
        (else
          (`PrimitiveComponent.SetEnableGravity` _dm_box false))))))

(event `Overlap`
  (params (OverlappedComponent :type "PrimitiveComponent Object Reference") (OtherActor :type "Actor Object Reference") (OtherComp :type "PrimitiveComponent Object Reference") (OtherBodyIndex :type Integer) (bFromSweep :type Boolean) (SweepResult :type "HitResult Structure (by ref)"))
  (if (== OtherActor (`GameplayStatics.GetPlayerPawn` 0))
    (goto _label)))

(event `self.ReceiveTick`
  (params (DeltaSeconds :type "Float (single-precision)")))

(fn `UserConstructionScript`
  (bind _box (`self.Box`))
  (`BoxComponent.SetBoxExtent` _box (`self.OverlapBoxExtent`) true)
  (`SceneComponent.SetVisibility` _box (`self.OverlapBoxVisible`) false))