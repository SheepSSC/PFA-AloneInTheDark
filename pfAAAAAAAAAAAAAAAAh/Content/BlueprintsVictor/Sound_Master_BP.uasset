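; Sound_Master_BP is an audio-reactive Blueprint that plays a sound on BeginPlay and drives an outline material parameter from it.
; The playback-percent callback converts progress to seconds and samples precomputed, normalized Constant-Q data for channel 0 at that time.
; Each band value is scaled and written to the same StepRadius0 scalar in the PC_Outline parameter collection, so only the last band's value remains.
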(event `self.ReceiveBeginPlay`
  (`AudioComponent.SetSound` (`self.Audio`) (`self.New Sound`))
  (set `self.Duration` (`SoundBase.Duration` (`self.New Sound`)))
  (add `AudioComponent.OnAudioPlaybackPercent` (`self.Audio`) (delegate `PlaybackChange`))
  (`AudioComponent.Play` (`self.Audio`) 0.0))

(event `PlaybackChange`
  (params (PlayingSoundWave :type "SoundWave Object Reference") (PlaybackPercent :type "Float (double-precision)"))
  (set `self.PlayedTime` (* PlaybackPercent (`self.Duration`)))
  (for _array_element (`ConstantQNRT.GetNormalizedChannelConstantQAtTime` (`self.Constant_ref`) (`self.PlayedTime`) 0)
    (`KismetMaterialLibrary.SetScalarParameterValue` "/Game/BlueprintsVictor/PC_Outline.PC_Outline" "StepRadius0" (* _array_element 200.0))))

(fn `UserConstructionScript`)